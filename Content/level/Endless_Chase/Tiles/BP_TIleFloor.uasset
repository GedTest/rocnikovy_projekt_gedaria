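; Floor tile for the Endless_Chase runner level, randomizing its obstacles and requesting the next tile as the player progresses.
; The construction script gathers two sets of three spawn transforms and adds a child actor at a random point from each.
; When 2D_Runner overlaps EndTrigger, it calls AddFloorTile on GameModeEndlessRunner.
; GetAttachTransform exposes the AttachPoint world transform.
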(event `self.EndTrigger.OnComponentBeginOverlap`
  (params (OverlappedComponent :type "PrimitiveComponent Object Reference") (OtherActor :type "Actor Object Reference") (OtherComp :type "PrimitiveComponent Object Reference") (OtherBodyIndex :type Integer) (bFromSweep :type Boolean) (SweepResult :type "HitResult Structure (by ref)"))
  (cast `/Game/level/Endless_Chase/2D_Runner` OtherActor)
  (bind _asgame_mode_endless_runner (cast `/Game/level/Endless_Chase/GameModeEndlessRunner` (`GameplayStatics.GetGameMode`)))
  (`/Game/level/Endless_Chase/GameModeEndlessRunner.AddFloorTile` _asgame_mode_endless_runner))

(fn `GetAttachTransform`
  (returns (AttachTransform :type "Transform Structure"))
  (return (`SceneComponent.K2_GetComponentToWorld` (`self.AttachPoint`))))

(fn `SetSpawnPoints`
  (set `self.SpawnPoints` (`|MakeArray` (`SceneComponent.GetRelativeTransform` (`self.SpawnPointRight`)) (`SceneComponent.GetRelativeTransform` (`self.SpanwPointLeft`)) (`SceneComponent.GetRelativeTransform` (`self.SpawnPoint`))))
  (set `self.Obstacle2SpawnPoints` (`|MakeArray` (`SceneComponent.GetRelativeTransform` (`self.Obstacle2`)) (`SceneComponent.GetRelativeTransform` (`self.obstacle2Left`)) (`SceneComponent.GetRelativeTransform` (`self.obstacle2Right`)))))

(fn `SpawnObstacle`
  (bind _obstacle2spawnpoints (`self.Obstacle2SpawnPoints`))
  (bind _spawnpoints (`self.SpawnPoints`))
  (`AddComponent|NODE_AddChildActorComponent-1` :`RelativeTransform` (`|GetArrayItem` _obstacle2spawnpoints (`KismetMathLibrary.RandomIntegerInRange` 0 (`KismetArrayLibrary.Array_LastIndex` _obstacle2spawnpoints))))
  (`AddComponent|NODE_AddChildActorComponent-0` :`RelativeTransform` (`|GetArrayItem` _spawnpoints (`KismetMathLibrary.RandomIntegerInRange` 0 (`KismetArrayLibrary.Array_LastIndex` _spawnpoints)))))

(fn `UserConstructionScript`
  (`self.SetSpawnPoints`)
  (`self.SpawnObstacle`))